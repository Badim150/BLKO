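; Game mode for a tower defense game, managing waves, score, tower selection and build mode.
; BeginPlay finds the finish line and enables a core spawner, whose wave number is mirrored on Tick.
; Purchases and minion rewards go through the player character, while spawners handle wave rushing and hard mode, or get disabled from wave 20.
; A synchronous navigation check from each spawner sets path availability when a path is partial.
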(event EventBeginPlay
  (bind _outactors (Actor|GetAllActorsOfClass "/Game/SpawnerAndFinishLine/FinishLine.FinishLine_C"))
  (Variables|Default|SetFinishLine (Utilities|Array|Get(acopy) _outactors))
  (bind _outactors_2 (Actor|GetAllActorsOfClass "/Game/SpawnerAndFinishLine/EnemySpawner.EnemySpawner_C"))
  (bind _output_get (Variables|Default|SetCoreSpawner (Utilities|Array|Get(acopy) _outactors_2)))
  (Class|Spawner|EnableSpawner _output_get)
  (Variables|Default|SetScore 0.0))

(event EventTick
  (params (DeltaSeconds :type Float%20%28single-precision%29))
  (Variables|Default|SetWave (Math|Conversions|ToFloat(Integer) (Variables|/Script/BLKO.Spawner|GetWaveNumber (Variables|Default|GetCoreSpawner)))))

(fn ConstructionScript)

(fn EnableBuildMode
  (params (Tower :type Integer))
  (Variables|Default|SetTowerToBuild Tower)
  (Variables|Default|SetBuildMode true))

(fn DisableBuildMode
  (Variables|Default|SetTowerToBuild -1)
  (Variables|Default|SetBuildMode false))

(fn SelectTower
  (params (Tower :type Puzzle%20Block%20Object%20Reference))
  (if (Utilities|IsValid (Variables|Default|GetHighlightedTower))
    (Default|DeSelectTower (Variables|Default|GetHighlightedTower)))
  (bind _output_get (Variables|Default|SetHighlightedTower Tower))
  (Utilities|IsValid _output_get
    (:Is%20Valid
      (Default|SelectTower _output_get))))

(fn CheckPathAvailability
  (bind _outactors (Actor|GetAllActorsOfClass "/Game/SpawnerAndFinishLine/EnemySpawner.EnemySpawner_C"))
  (for _array_element _outactors
    (bind _returnvalue (Class|NavigationSystem|FindPathtoActorSynchronously (Transformation|GetActorLocation _array_element) (Variables|Default|GetFinishLine) 5e+01))
    (if (Class|NavigationPath|IsPartial _returnvalue)
      (LocalVariables|SetisPathAvailable true)))
  (return (LocalVariables|GetisPathAvailable)))

(fn BuyTower
  (bind _asblkoplayer_character (Utilities|Casting|CastToBLKOPlayerCharacter (Game|GetPlayerCharacter 0)))
  (switch int (Variables|Default|GetTowerToBuild)
    (:0
      (Default|BuyTower _asblkoplayer_character 1e+02))
    (:1
      (Default|BuyTower _asblkoplayer_character 1e+02))
    (:2
      (Default|BuyTower _asblkoplayer_character 2e+02)))
  (CallFunction|DisableBuildMode))

(fn CashMinion
  (params (MinionWorth :type Float%20%28single-precision%29))
  (Variables|Default|SetScore (+ MinionWorth (Variables|Default|GetScore)))
  (bind _asblkoplayer_character (Utilities|Casting|CastToBLKOPlayerCharacter (Game|GetPlayerCharacter 0)))
  (Default|SellTower _asblkoplayer_character MinionWorth))

(fn RushWave
  (bind _outactors (Actor|GetAllActorsOfClass "/Game/SpawnerAndFinishLine/EnemySpawner.EnemySpawner_C"))
  (for _array_element _outactors
    (if (Variables|/Script/BLKO.Spawner|GetEnabled _array_element)
      (Class|Spawner|RushWave _array_element))))

(fn EnableHardMode
  (if (>= (Variables|Default|GetWave) 2e+01)
    (bind _outactors (Actor|GetAllActorsOfClass "/Game/SpawnerAndFinishLine/EnemySpawner.EnemySpawner_C"))
    (Class|Spawner|DisableSpawner _outactors)
    (else
      (bind _outactors_2 (Actor|GetAllActorsOfClass "/Game/SpawnerAndFinishLine/EnemySpawner.EnemySpawner_C"))
      (Class|Spawner|HardMode _outactors_2 11)
      (Class|Spawner|EnableSpawner _outactors_2 11))))