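; Game mode for a tower defense game, tracking score, wave number, tower build and selection state, and game over after repeated boss deaths.
; Tower purchases and minion rewards route money through the player character, while the wave count mirrors the first enemy spawner.
; Functions broadcast wave rushes and hard mode to all spawners and run navigation path checks from them to the finish line.
; SaveScore inserts scores by rank into a SaveGame slot.
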(event Custom|GameOver?
  (bind _deadbosses (Variables|Default|GetDeadBosses))
  (if (>= _deadbosses 3)
    (CallFunction|EndGame)
    (else
      (Math|Integer|IncrementInt _deadbosses))))

(event EventBeginPlay
  (bind _outactors (Actor|GetAllActorsOfClass "/Game/Import/SpawnerAndFinishLine/FinishLine.FinishLine_C"))
  (Variables|Default|SetFinishLine (Utilities|Array|Get(acopy) _outactors))
  (bind _outactors_2 (Actor|GetAllActorsOfClass "/Game/Import/SpawnerAndFinishLine/EnemySpawner.EnemySpawner_C"))
  (Variables|Default|SetCoreSpawner (Utilities|Array|Get(acopy) _outactors_2))
  (Variables|Default|SetScore 0.0))

(event EventTick
  (params (DeltaSeconds :type Float%20%28single-precision%29))
  (Variables|Default|SetWave (Math|Conversions|ToFloat(Integer) (Variables|/Script/BLKO.Spawner|GetWaveNumber (Variables|Default|GetCoreSpawner)))))

(fn ConstructionScript)

(fn EnableBuildMode
  (params (Tower :type Integer))
  (Variables|Default|SetTowerToBuild Tower)
  (Variables|Default|SetBuildMode true))

(fn DisableBuildMode
  (Variables|Default|SetTowerToBuild -1)
  (Variables|Default|SetBuildMode false))

(fn SelectTower
  (params (Tower :type Puzzle%20Block%20Object%20Reference))
  (if (Utilities|IsValid (Variables|Default|GetHighlightedTower))
    (Default|DeSelectTower (Variables|Default|GetHighlightedTower)))
  (bind _output_get (Variables|Default|SetHighlightedTower Tower))
  (Utilities|IsValid _output_get
    (:Is%20Valid
      (Default|SelectTower _output_get))))

(fn CheckPathAvailability
  (bind _outactors (Actor|GetAllActorsOfClass "/Game/Import/SpawnerAndFinishLine/EnemySpawner.EnemySpawner_C"))
  (for _array_element _outactors
    (bind _returnvalue (Class|NavigationSystem|FindPathtoActorSynchronously (Transformation|GetActorLocation _array_element) (Variables|Default|GetFinishLine) 5e+01))
    (if (Class|NavigationPath|IsPartial _returnvalue)
      (LocalVariables|SetisPathAvailable true)))
  (return (LocalVariables|GetisPathAvailable)))

(fn BuyTower
  (bind _asblkoplayer_character (Utilities|Casting|CastToBLKOPlayerCharacter (Game|GetPlayerCharacter 0)))
  (switch int (Variables|Default|GetTowerToBuild)
    (:0
      (Default|BuyTower _asblkoplayer_character 1e+02))
    (:1
      (Default|BuyTower _asblkoplayer_character 1e+02))
    (:2
      (Default|BuyTower _asblkoplayer_character 1.5e+02)))
  (CallFunction|DisableBuildMode))

(fn CashMinion
  (params (MinionWorth :type Float%20%28single-precision%29))
  (Variables|Default|SetScore (+ MinionWorth (Variables|Default|GetScore)))
  (bind _asblkoplayer_character (Utilities|Casting|CastToBLKOPlayerCharacter (Game|GetPlayerCharacter 0)))
  (Default|SellTower _asblkoplayer_character MinionWorth))

(fn RushWave
  (bind _outactors (Actor|GetAllActorsOfClass "/Game/Import/SpawnerAndFinishLine/EnemySpawner.EnemySpawner_C"))
  (for _array_element _outactors
    (Class|Spawner|RushWave _array_element)))

(fn EnableHardMode
  (if (not (Variables|Default|GetHardModeON))
    (Variables|Default|SetHardModeON true)
    (bind _outactors (Actor|GetAllActorsOfClass "/Game/Import/SpawnerAndFinishLine/EnemySpawner.EnemySpawner_C"))
    (for _array_element _outactors
      (if (Variables|/Script/BLKO.Spawner|GetEnabled _array_element)
        (Class|Spawner|DisableSpawner _array_element)
        (else
          (Class|Spawner|EnableSpawner _array_element 10)
          (Class|Spawner|HardMode _array_element 10))))))

(fn SaveScore
  (params (Name :type Text))
  (bind _temp (LocalVariables|GetTemp))
  (bind _score (Variables|Default|GetScore))
  (bind _returnvalue (SaveGame|LoadGamefromSlot "scoreSave"))
  (bind _asscore_save (Utilities|Casting|CastToscoreSave _returnvalue)
    (:then
      (for _array_element (Variables|/Game/GameBlueprints/Widgets/ScoreBoard/scoreSave.scoreSave_C|GetPlayerScores _asscore_save)
        (Utilities|FlowControl|Sequence
          (:then_0
            (if (<= (.Score (Utilities|Struct|BreakPlayerScore _array_element)) _score)
              (Utilities|FlowControl|DoOnce false
                (:Completed
                  (Utilities|Array|Add _temp (Utilities|Struct|MakePlayerScore Name _score (Class|KismetMathLibrary|GetDate)))
                  (Development|PrintString (Utilities|String|Append "saved: " (Utilities|String|ToString(Text) Name) " score: " (Utilities|String|ToString(Float) _score)))))))
          (:then_1
            (Utilities|Array|Add _temp _array_element))))
      (bind _returnvalue_2 (SaveGame|CreateSaveGameObject "/Game/GameBlueprints/Widgets/ScoreBoard/scoreSave.scoreSave_C" :!label _label))
      (bind _asscore_save_2 (Utilities|Casting|CastToscoreSave _returnvalue_2))
      (Variables|/Game/GameBlueprints/Widgets/ScoreBoard/scoreSave.scoreSave_C|SetPlayerScores _asscore_save_2 (LocalVariables|GetTemp))
      (SaveGame|SaveGametoSlot _returnvalue_2 "scoreSave"))
    (:CastFailed
      (Utilities|FlowControl|Sequence
        (:then_0
          (Utilities|FlowControl|DoOnce false
            (:Completed
              (Utilities|Array|Add _temp (Utilities|Struct|MakePlayerScore Name _score (Class|KismetMathLibrary|GetDate)))
              (Development|PrintString (Utilities|String|Append "saved: " (Utilities|String|ToString(Text) Name) " score: " (Utilities|String|ToString(Float) _score))))))
        (:then_1
          (goto _label))))))

(fn EndGame
  (bind _returnvalue (UserInterface|CreateWidget "/Game/GameBlueprints/Widgets/GameOverMenu.GameOverMenu_C"))
  (Input|SetInputModeUIOnly (Game|GetPlayerController 0) _returnvalue "DoNotLock")
  (UserInterface|Viewport|AddtoViewport _returnvalue 0)
  (Game|SetGamePaused true))