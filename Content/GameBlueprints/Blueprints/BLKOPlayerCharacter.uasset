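; BLKOPlayerCharacter is the tower defense player character, holding gold and base health and handling build, cancel and pause input.
; On BeginPlay it creates the HUD and caches BLKOGameMode, which it drives to toggle build mode, set the tower to build and deselect highlighted towers.
; Escape cancels build mode or opens a reused pause menu.
; Buy and sell functions adjust gold, while scaled damage lowers base health and ends the game at zero.
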(event Custom|Cancel
  (bind _gamemode (Variables|Default|GetGameMode))
  (if (Variables|/Game/GameBlueprints/Blueprints/BLKOGameMode.BLKOGameMode_C|GetBuildMode _gamemode)
    (Default|DisableBuildMode _gamemode)
    (Variables|/Script/Engine.PlayerController|SetbEnableMouseOverEvents (Game|GetPlayerController 0) true)
    (else
      (Default|DeSelectTower (Variables|/Game/GameBlueprints/Blueprints/BLKOGameMode.BLKOGameMode_C|GetHighlightedTower _gamemode))
      (Utilities|FlowControl|Delay 0.1)
      (Variables|/Game/GameBlueprints/Blueprints/BLKOGameMode.BLKOGameMode_C|SetHighlightedTower _gamemode 0))))

(event Custom|BuildTower
  (params (Tower :type Integer))
  (bind _gamemode (Variables|Default|GetGameMode))
  (Default|EnableBuildMode _gamemode)
  (Default|SelectTower _gamemode)
  (Variables|/Script/Engine.PlayerController|SetbEnableMouseOverEvents (Game|GetPlayerController 0) true)
  (Variables|/Game/GameBlueprints/Blueprints/BLKOGameMode.BLKOGameMode_C|SetTowerToBuild _gamemode Tower))

(event EventBeginPlay
  ;[1 1 1] HUD init
  (bind _returnvalue (UserInterface|CreateWidget "/Game/GameBlueprints/Widgets/BLKOHUD.BLKOHUD_C"))
  (bind _output_get (Variables|Default|SetHUD_reference _returnvalue))
  (UserInterface|Viewport|AddtoViewport _output_get 0)
  (Variables|/Script/Engine.PlayerController|SetCurrentMouseCursor (Game|GetPlayerController 0) "Default")
  (bind _asblkogame_mode (Utilities|Casting|CastToBLKOGameMode (Game|GetGameMode)))
  (Variables|Default|SetGameMode _asblkogame_mode))

(event Input|KeyboardEvents|Escape
  (params (Key :type Key%20Structure :default "AnyKey"))
  (:Pressed
    (if (Variables|/Game/GameBlueprints/Blueprints/BLKOGameMode.BLKOGameMode_C|GetBuildMode (Variables|Default|GetGameMode))
      (CallFunction|Cancel)
      (else
        (Utilities|IsValid (Variables|Default|GetPause%20Menu%20Reference)
          (:Is%20Valid
            _)
          (:Is%20Not%20Valid
            (bind _returnvalue (UserInterface|CreateWidget "/Game/GameBlueprints/Widgets/PauseMenu.PauseMenu_C"))
            (Variables|Default|SetPause%20Menu%20Reference _returnvalue)))
        (Input|SetInputModeUIOnly (Game|GetPlayerController 0) (Variables|Default|GetPause%20Menu%20Reference) "DoNotLock")
        (UserInterface|Viewport|AddtoViewport (Variables|Default|GetPause%20Menu%20Reference) 0)
        (Game|SetGamePaused true)))))

(fn ConstructionScript)

(fn SellTower
  (params (gold :type Float%20%28single-precision%29))
  (Variables|Default|SetPlayerGold (+ gold (Variables|Default|GetPlayerGold))))

(fn BuyTower
  (params (gold :type Float%20%28single-precision%29))
  (Variables|Default|SetPlayerGold (- (Variables|Default|GetPlayerGold) gold)))

(fn TakeDamage
  (params (Damage :type Float%20%28single-precision%29))
  (bind _output_get (Variables|Default|SetBaseHealth (- (Variables|Default|GetBaseHealth) (* Damage 0.1))))
  (if (<= _output_get 0.0)
    (Default|EndGame (Variables|Default|GetGameMode))))